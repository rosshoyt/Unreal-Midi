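; Music visualizer controller that makes a grid of note cubes react to note messages received over local OSC.
; On BeginPlay it spawns BP_NoteCube actors in a square-style grid and starts an OSC server.
; Each message's first integer indexes LastNoteHeatmap, storing that note's last game time, and is printed with its address.
; Tick stretches cubes vertically for one second after their note and otherwise resets their scale.
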(event Custom|OnMsgReceived
  (params (Message :type OSC%20Message%20Structure%20%28by%20ref%29) (IPAddress :type String) (Port :type Integer))
  ;[1 1 1] Startup, Binding to Any MIDI Message
  (bind _returnvalue (Class|OSCManager|GetOSCMessageAddress Message))
  (bind _returnvalue_2 (Class|OSCManager|GetOSCAddressFullPath _returnvalue))
  (bind _value (Class|OSCManager|GetInt32 Message))
  (Utilities|Array|SetArrayElem (Variables|Default|GetLastNoteHeatmap) _value (Utilities|Time|GetGameTimeinSeconds))
  (Development|PrintString (Utilities|String|Append "Address: " _returnvalue_2 "Value: " (Utilities|String|ToString(Integer) _value)) true false))

(event EventTick
  (params (DeltaSeconds :type Float%20%28single-precision%29))
  (CallFunction|UpdateGrid DeltaSeconds))

(event EventBeginPlay
  ;[1 1 1] Startup, Binding to Any MIDI Message
  (CallFunction|SpawnGrid)
  (bind _returnvalue (Class|OSCManager|CreateOSCServer "127.0.0.1" 1312 false true "" 0))
  (EventDispatchers|AssignOnOscMessageReceived _returnvalue (delegate Custom|OnMsgReceived)))

(fn ConstructionScript)

(fn SpawnGrid
  (bind _distance (Variables|Default|GetDistance))
  (for _index (range 0 (- (Variables|Default|GetNumber%20of%20Cubes) 1))
    (Utilities|Array|Add (Variables|Default|GetLastNoteHeatmap) -1e+06) ; Fill Last Note Heatmap
    (bind _returnvalue (Game|SpawnActorfromClass "/Game/blueprints/BP_NoteCube.BP_NoteCube_C" (Math|Transform|MakeTransform (Math|Vector|MakeVector (* (Variables|Default|GetRow) _distance) (* (Variables|Default|GetColumn) _distance) 0.0) "0, 0, 0" "1,1,1") "AlwaysSpawn" 0 0))
    (Utilities|Array|Add (Variables|Default|GetBP_NoteCubeArray) _returnvalue)
    (Math|Integer|IncrementInt (Variables|Default|GetRow)
      (:%20%20
        (if (== (Variables|Default|GetRow) (Math|Float|Truncate (Math|Float|Sqrt (Math|Conversions|ToFloat(Integer) (Variables|Default|GetNumber%20of%20Cubes)))))
          (Math|Integer|IncrementInt (Variables|Default|GetColumn)
            (:%20%20
              (Variables|Default|SetRow 0))))))))

(fn UpdateGrid
  (params (DeltaSeconds :type Float%20%28single-precision%29))
  (for (_array_element _array_index) (Variables|Default|GetBP_NoteCubeArray)
    (if (> 1.0 (- (Utilities|Time|GetGameTimeinSeconds) (Utilities|Array|Get(acopy) (Variables|Default|GetLastNoteHeatmap) _array_index))) ; Check if less than 1 second since note
      (Transformation|SetActorScale3D _array_element (Math|Vector|MakeVector 1.0 1.0 5.0))
      (else
        (Transformation|SetActorScale3D _array_element (Math|Vector|MakeVector 1.0 1.0 1.0))))))