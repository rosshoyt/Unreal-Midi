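; BP_EQController1 spawns a flat grid of BP_NoteCube actors when play begins.
; SpawnGrid places NumberOfCubes cubes spaced by Distance in world coordinates, wrapping each row at the truncated square root of the count for a roughly square layout.
; Cubes share a fixed tilt, always spawn regardless of collision, and are stored in BPNoteCubeArray.
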(event EventBeginPlay
  (CallFunction|SpawnGrid))

(fn ConstructionScript)

(fn SpawnGrid
  (bind _distance (Variables|Default|GetDistance))
  (for _index (range 0 (- (Variables|Default|GetNumber%20of%20Cubes) 1))
    (bind _returnvalue (Game|SpawnActorfromClass "/Game/blueprints/BP_NoteCube.BP_NoteCube_C" (Math|Transform|MakeTransform (Math|Vector|MakeVector (* (Variables|Default|GetRow) _distance) (* (Variables|Default|GetColumn) _distance) 0.0) "-5.000000,10.000000,10.000000" "1,1,1") "AlwaysSpawn" 0 0))
    (Utilities|Array|Add (Variables|Default|GetBP_NoteCubeArray) _returnvalue)
    (Math|Integer|IncrementInt (Variables|Default|GetRow)
      (:%20%20
        (if (== (Variables|Default|GetRow) (Math|Float|Truncate (Math|Float|Sqrt (Math|Conversions|ToFloat(Integer) (Variables|Default|GetNumber%20of%20Cubes)))))
          (Math|Integer|IncrementInt (Variables|Default|GetColumn)
            (:%20%20
              (Variables|Default|SetRow 0))))))))